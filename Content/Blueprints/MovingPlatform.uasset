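; Paper2D moving platform that shuttles a sprite between its origin and a configurable EndLocation.
; A timeline lerps the relative location without sweep, then pauses briefly at each end and restarts in the opposite direction.
; When Bull_Character overlaps the Bottom component and the timeline is active, it calls Play if already playing, otherwise Reverse.
; The construction script applies the configured PlatformSprite.
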(event OnComponentBeginOverlap(Bottom)
  (params (OtherActor :type Actor%20Object%20Reference) (OtherComp :type Primitive%20Component%20Object%20Reference) (OtherBodyIndex :type Integer) (bFromSweep :type Boolean) (SweepResult :type Hit%20Result%20Structure%20%28by%20ref%29))
  (bind _platformtimeline (Variables|Default|GetPlatformTimeline))
  (Utilities|Casting|CastToBull_Character OtherActor)
  (if (Components|Activation|IsActive _platformtimeline)
    (if (Audio|Components|Audio|IsPlaying _platformtimeline)
      (bind (_direction _timeline) (Timeline|PlatformTimeline Play)
        (:Update
          (Transformation|SetRelativeLocation (Variables|Default|GetPlatform) (Math|Vector|Lerp(Vector) "0, 0, 0" (Variables|Default|GetEndLocation) _timeline) false))
        (:Finished
          (Utilities|FlowControl|Delay 2.0)
          (switch Utilities|FlowControl|Switch|SwitchonETimelineDirection _direction
            (:Forward
              (Timeline|PlatformTimeline ReverseFromEnd))
            (:Backward
              (Timeline|PlatformTimeline PlayFromStart)))))
      (else
        (Timeline|PlatformTimeline Reverse)))))

(fn ConstructionScript
  (Rendering|Components|Sprite|SetSprite (Variables|Default|GetPlatform) (Variables|Default|GetPlatformSprite)))