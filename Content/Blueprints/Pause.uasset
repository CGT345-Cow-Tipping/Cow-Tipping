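; Pause is an actor that toggles the game's paused state when P is pressed or TogglePause is called.
; On BeginPlay it enables input from the first player controller and registers itself as PauseBP on the CTHUD.
; Each toggle triggers the HUD's pause message, switches mouse cursor and click events on while paused, and flips the Pause flag.
; GetHealth and SaveData are empty stubs.
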(event EventBeginPlay
  (bind _returnvalue (Game|GetPlayerController 0))
  (Variables|Default|SetPlayerController _returnvalue)
  (Input|EnableInput (Variables|Default|GetPlayerController))
  (bind _ascthud_c (Utilities|Casting|CastToCTHUD (HUD|GetHUD _returnvalue)))
  (Variables|/Game/Blueprints/CTHUD.CTHUD_C|SetPauseBP _ascthud_c self))

(event EventTogglePause
  (bind _playercontroller (Variables|Default|GetPlayerController))
  (bind _playercontroller_2 (Variables|Default|GetPlayerController))
  (Class|HUDInterface|TogglePause(Message) (HUD|GetHUD (Variables|Default|GetPlayerController)))
  (if (Variables|Default|GetPause)
    (Variables|/Script/Engine.PlayerController|SetbShowMouseCursor _playercontroller_2 false)
    (Variables|/Script/Engine.PlayerController|SetbEnableClickEvents _playercontroller_2 false)
    (else
      (Variables|/Script/Engine.PlayerController|SetbShowMouseCursor _playercontroller true)
      (Variables|/Script/Engine.PlayerController|SetbEnableClickEvents _playercontroller true)))
  (Game|SetGamePaused (not (Variables|Default|GetPause)))
  (Variables|Default|SetPause (not (Variables|Default|GetPause))))

(event Input|KeyboardEvents|P
  (bind _playercontroller (Variables|Default|GetPlayerController))
  (bind _playercontroller_2 (Variables|Default|GetPlayerController))
  (:Pressed
    (Class|HUDInterface|TogglePause(Message) (HUD|GetHUD (Variables|Default|GetPlayerController)))
    (if (Variables|Default|GetPause)
      (Variables|/Script/Engine.PlayerController|SetbShowMouseCursor _playercontroller_2 false)
      (Variables|/Script/Engine.PlayerController|SetbEnableClickEvents _playercontroller_2 false)
      (else
        (Variables|/Script/Engine.PlayerController|SetbShowMouseCursor _playercontroller true)
        (Variables|/Script/Engine.PlayerController|SetbEnableClickEvents _playercontroller true)))
    (Game|SetGamePaused (not (Variables|Default|GetPause)))
    (Variables|Default|SetPause (not (Variables|Default|GetPause)))))

(fn ConstructionScript)

(fn GetHealth
  (return 0))

(fn SaveData
  (return 0))