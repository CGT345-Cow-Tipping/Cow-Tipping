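; Paper2D side-scrolling enemy AI with Blacksmith, Clown and Redneck variants, destroyed by a player attack at close range.
; The construction script orders two patrol points and sets each type's flipbooks and ranges.
; Tick chooses attack, follow within the patrol bounds, or patrol, based on player distance.
; Flipbook playback windows with DoOnce gates time melee hits or projectile throws, arced with fixed vertical speed and distance-scaled horizontal speed.
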(event EventPlayerAttack
  (params (Damage :type Integer) (Range :type Float%20%28single-precision%29))
  (bind _returnvalue (Game|GetPlayerCharacter 0))
  (bind _returnvalue_2 (Transformation|GetActorLocation))
  (bind _returnvalue_3 (Transformation|GetActorLocation _returnvalue))
  (bind (_x _y _z) (Math|Vector|BreakVector _returnvalue_2))
  (bind (_x_2 _y_2 _z_2) (Math|Vector|BreakVector _returnvalue_3))
  (if (and (Math|Float|InRange(Float) (- _x_2 _x) -1.7e+02 1.7e+02) (Math|Float|InRange(Float) (- _z_2 _z) -1e+02 1e+02))
    (Actor|DestroyActor)))

(event EventTick
  (params (DeltaSeconds :type Float%20%28single-precision%29))
  (bind _returnvalue (Game|GetPlayerCharacter 0))
  (bind _returnvalue_2 (Transformation|GetActorLocation))
  (bind _returnvalue_3 (Game|GetPlayerCharacter 0))
  (bind _returnvalue_4 (Transformation|GetActorLocation))
  (bind _attackrange (Variables|Default|GetAttackRange))
  (bind _followrange (Variables|Default|GetFollowRange))
  (bind _returnvalue_5 (Transformation|GetActorLocation _returnvalue))
  (bind (_x _y _z) (Math|Vector|BreakVector _returnvalue_2))
  (bind _returnvalue_6 (Transformation|GetActorLocation _returnvalue_3))
  (bind (_x_2 _y_2 _z_2) (Math|Vector|BreakVector _returnvalue_4))
  (bind (_x_3 _y_3 _z_3) (Math|Vector|BreakVector _returnvalue_5))
  (bind (_x_4 _y_4 _z_4) (Math|Vector|BreakVector _returnvalue_6))
  (bind _returnvalue_7 (- _x_3 _x))
  (bind _returnvalue_8 (- _z_3 _z))
  (bind _returnvalue_9 (Math|Float|InRange(Float) _returnvalue_8 -7e+02 7e+02))
  (if (and (Math|Float|InRange(Float) _returnvalue_7 _attackrange (Math|Float|Absolute(Float) _attackrange)) _returnvalue_9)
    ;[1 1 1] Face the player and attack
    (CallFunction|ChangeFlipbook "Attack")
    (Utilities|CheckPlayertoEnemy
      (:Right
        (Transformation|SetActorRelativeRotation "0,0.000000, 0")
        (Variables|Default|SetDirection "Right"))
      (:Left
        (Transformation|SetActorRelativeRotation "0.000000,180.000000, 0")
        (Variables|Default|SetDirection "Left")))
    (switch Utilities|FlowControl|Switch|SwitchonEnemyTypeEnum (Variables|Default|GetEnemyType)
      (:NewEnumerator0
        ;[1 1 1] Melee Attack (blacksmith)
        (if (and (Math|Float|InRange(Float) (- _x_4 _x_2) -1.1e+02 1.1e+02) (Math|Float|InRange(Float) (- _z_4 _z_2) -1e+02 1e+02))
          (if (Math|Float|InRange(Float) (Components|Timeline|GetPlaybackPosition (Variables|Default|GetSprite)) 0.4 0.5 true false)
            (Utilities|FlowControl|DoOnce false :!label _label
              (:Completed
                (Class|DamageInterface|HitPlayer(Message) (Game|GetPlayerCharacter 0) 3)
                (Class|DamageInterface|HitPlayer(Message) (HUD|GetHUD (Game|GetPlayerController 0)) 3)))
            (else
              (goto _label Reset)))))
      (:NewEnumerator1
        (if (Math|Float|InRange(Float) (Components|Timeline|GetPlaybackPosition (Variables|Default|GetSprite)) 0.5 0.6 true false)
          (Utilities|FlowControl|DoOnce false :!label _label_2
            (:Completed
              (CallFunction|ThrowProjectile)))
          (else
            (goto _label_2 Reset))))
      (:NewEnumerator2
        (if (Math|Float|InRange(Float) (Components|Timeline|GetPlaybackPosition (Variables|Default|GetSprite)) 0.66 0.7 true false)
          (Utilities|FlowControl|DoOnce false :!label _label_3
            (:Completed
              (CallFunction|ThrowProjectile)))
          (else
            (goto _label_3 Reset)))))
    (elif (and _returnvalue_9 (Math|Float|InRange(Float) _returnvalue_7 _followrange (Math|Float|Absolute(Float) _followrange)))
      ;[1 1 1] Follow the player until a target point is reached
      (Utilities|CheckPlayertoEnemy
        (:Right
          (Transformation|SetActorRelativeRotation "0,0.000000, 0")
          (Math|Float|CompareFloat (- (.X (Math|Vector|BreakVector (Variables|Default|GetRightPoint))) (.X (Math|Vector|BreakVector (Transformation|GetActorLocation)))) 0.0
            (:>
              (CallFunction|ChangeFlipbook "Walk")
              (Pawn|Input|AddMovementInput "1.000000, 0, 0" 1.0)
              (Variables|Default|SetDirection "Right"))
            (:<
              (CallFunction|ChangeFlipbook "Idle"))))
        (:Left
          (Transformation|SetActorRelativeRotation "0,180.000000, 0")
          (Math|Float|CompareFloat (- (.X (Math|Vector|BreakVector (Variables|Default|GetLeftPoint))) (.X (Math|Vector|BreakVector (Transformation|GetActorLocation)))) 0.0
            (:>
              (CallFunction|ChangeFlipbook "Idle"))
            (:<
              (CallFunction|ChangeFlipbook "Walk")
              (Pawn|Input|AddMovementInput "1.000000, 0, 0" -1.0)
              (Variables|Default|SetDirection "Left")))))
      (elif (Utilities|Name|Equal(Name) (Variables|Default|GetDirection) "Left")
        ;[1 1 1] Patrol between the target points
        (Pawn|Input|AddMovementInput "1.000000, 0, 0" -1.0)
        (if (> (- (.X (Math|Vector|BreakVector (Variables|Default|GetLeftPoint))) (.X (Math|Vector|BreakVector (Transformation|GetActorLocation)))) 0.0)
          (Transformation|SetActorRelativeRotation "0,0.000000, 0")
          (Variables|Default|SetDirection "Right"))
        (else
          (Pawn|Input|AddMovementInput "1.000000, 0, 0" 1.0)
          (if (< (- (.X (Math|Vector|BreakVector (Variables|Default|GetRightPoint))) (.X (Math|Vector|BreakVector (Transformation|GetActorLocation)))) 0.0)
            (Transformation|SetActorRelativeRotation "0,180.000000, 0")
            (Variables|Default|SetDirection "Left")))))))

(fn ConstructionScript
  (bind _pointa (Variables|Default|GetPointA))
  (bind _pointb (Variables|Default|GetPointB))
  (bind _returnvalue (Transformation|GetActorLocation _pointa))
  (bind _returnvalue_2 (Transformation|GetActorLocation _pointb))
  (Math|Float|CompareFloat (.X (Math|Vector|BreakVector _returnvalue)) (.X (Math|Vector|BreakVector _returnvalue_2))
    (:>
      (Variables|Default|SetRightPoint _returnvalue)
      (Variables|Default|SetLeftPoint _returnvalue_2))
    (:<
      (Variables|Default|SetRightPoint _returnvalue_2)
      (Variables|Default|SetLeftPoint _returnvalue)))
  (switch Utilities|FlowControl|Switch|SwitchonEnemyTypeEnum (Variables|Default|GetEnemyType)
    (:NewEnumerator0
      (Variables|Default|SetWalkFlipbook "/Game/Sprites/Characters/BlacksmithWalk.BlacksmithWalk")
      (Variables|Default|SetIdleFlipbook "/Game/Sprites/Characters/BlacksmithIdle.BlacksmithIdle")
      (Variables|Default|SetAttackFlipbook "/Game/Sprites/Characters/BlacksmithAttack.BlacksmithAttack")
      (Variables|Default|SetAttackRange -1.7e+02)
      (Variables|Default|SetFollowRange -5e+02))
    (:NewEnumerator1
      (Variables|Default|SetWalkFlipbook "/Game/Sprites/Characters/ClownWalk.ClownWalk")
      (Variables|Default|SetIdleFlipbook "/Game/Sprites/Characters/ClownIdle.ClownIdle")
      (Variables|Default|SetAttackFlipbook "/Game/Sprites/Characters/ClownAttack.ClownAttack")
      (Variables|Default|SetAttackRange -8e+02)
      (Variables|Default|SetFollowRange -1e+03))
    (:NewEnumerator2
      (Variables|Default|SetWalkFlipbook "/Game/Sprites/Characters/RedNeckWalk.RedNeckWalk")
      (Variables|Default|SetIdleFlipbook "/Game/Sprites/Characters/RedNeckIdle.RedNeckIdle")
      (Variables|Default|SetAttackFlipbook "/Game/Sprites/Characters/RedNeckAttack.RedNeckAttack")
      (Variables|Default|SetAttackRange -8e+02)
      (Variables|Default|SetFollowRange -1e+03)))
  (Sprite|SetFlipbook (Variables|Default|GetSprite) (Variables|Default|GetWalkFlipbook)))

(fn ChangeFlipbook
  (params (New :type Name))
  (if (not (Utilities|Name|Equal(Name) New (Variables|Default|GetActiveFlipbook)))
    (switch name New
      (:Walk
        (LocalVariables|SetNewFlipbook (Variables|Default|GetWalkFlipbook)))
      (:Idle
        (LocalVariables|SetNewFlipbook (Variables|Default|GetIdleFlipbook)))
      (:attack
        (LocalVariables|SetNewFlipbook (Variables|Default|GetAttackFlipbook))))
    (Sprite|SetFlipbook (Variables|Default|GetSprite) (LocalVariables|GetNewFlipbook))
    (Variables|Default|SetActiveFlipbook New)))

(fn ThrowProjectile
  (bind _returnvalue (Game|GetPlayerCharacter 0))
  (bind _returnvalue_2 (Transformation|GetActorLocation))
  (bind _returnvalue_3 (Transformation|GetActorLocation _returnvalue))
  (bind (_x _y _z) (Math|Vector|BreakVector _returnvalue_3))
  (if (Utilities|Enum|Equal(Enum) (Variables|Default|GetEnemyType) "NewEnumerator1")
    (LocalVariables|SetProjectileOffset "100.000000,0.000000,40.000000")
    (else
      (LocalVariables|SetProjectileOffset "100.000000,0.000000,70.000000")))
  (if (<= (- (.X (Math|Vector|BreakVector _returnvalue_2)) _x) 0.0)
    (LocalVariables|SetProjectileSpawnLocation (+ _returnvalue_2 (LocalVariables|GetProjectileOffset)))
    (else
      (LocalVariables|SetProjectileSpawnLocation (+ _returnvalue_2 (* (LocalVariables|GetProjectileOffset) "-1.000000,1.000000,1.000000")))))
  (bind _returnvalue_4 (Game|SpawnActorfromClass "/Game/Blueprints/Projectile.Projectile_C" (Math|Transform|MakeTransform (LocalVariables|GetProjectileSpawnLocation) "0, 0, 0" "5.000000,5.000000,5.000000") false))
  (LocalVariables|SetProjectileObject _returnvalue_4)
  (Game|Components|ProjectileMovement|SetVelocityinLocalSpace (Variables|/Game/Blueprints/Projectile.Projectile_C|GetProjectileMovement (LocalVariables|GetProjectileObject)) (Math|Vector|MakeVector (/ (- _x (.X (Math|Vector|BreakVector (+ _returnvalue_2 (LocalVariables|GetProjectileOffset))))) 2.0) 0.0 (+ (/ (* 1e+03 2.0) 2.0) (* 2.45 2.0)))))