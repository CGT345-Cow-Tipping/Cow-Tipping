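; CTGameMode is the CowTipping game mode, handling save data and next-level progress.
; LoadSave creates a fresh CowTipping_Save on the first level or when none exists, otherwise loads the "save" slot.
; It sets NextLevel to one past a non-zero current level and sends the object to the HUD.
; SaveObject gets the save data back from the HUD and writes it to that slot.
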(event EventLoadSave
  (params (FirstLevel :type Boolean) (CurrentLevel :type Integer))
  (bind _returnvalue (SaveGame|DoesSaveGameExist "save"))
  (if _returnvalue
    (if FirstLevel
      (bind _returnvalue_2 (SaveGame|CreateSaveGameObject "/Game/Blueprints/CowTipping_Save.CowTipping_Save_C" :!label _label))
      (bind _ascowtipping_save_c (Utilities|Casting|CastToCowTipping_Save _returnvalue_2))
      (Variables|Default|SetSaveGameObject _ascowtipping_save_c)
      (else
        (bind _returnvalue_3 (SaveGame|LoadGamefromSlot "save"))
        (bind _ascowtipping_save_c_2 (Utilities|Casting|CastToCowTipping_Save _returnvalue_3))
        (Variables|Default|SetSaveGameObject _ascowtipping_save_c_2)))
    (else
      (goto _label)))
  (if (== CurrentLevel 0)
    _
    (else
      (Variables|/Game/Blueprints/CowTipping_Save.CowTipping_Save_C|SetNext%20Level (Variables|Default|GetSaveGameObject) (+ CurrentLevel 1))))
  (Class|SaveInterface|SendSave(Message) (HUD|GetHUD (Game|GetPlayerController 0)) (Variables|Default|GetSaveGameObject)))

(event EventSaveObject
  (bind _save (Class|HUDInterface|SaveData(Message) (HUD|GetHUD (Game|GetPlayerController 0))))
  (SaveGame|SaveGametoSlot _save "save"))

(fn ConstructionScript)