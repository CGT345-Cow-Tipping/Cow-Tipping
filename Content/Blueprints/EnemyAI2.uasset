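; Paper2D side-scrolling enemy AI that walks along X and switches to chasing the player with an attack flipbook when in range.
; Construction Script orders PointA/PointB into left/right bounds and picks flipbooks by EnemyType (only Blacksmith is handled).
; Tick checks XZ distance, sets flipbook and Direction, limits chase near the bounds, and calls Move to rotate and add input.
; The Timeline-based patrol turnarounds at the points are disconnected, so never run.
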(event EventTick
  (params (DeltaSeconds :type Float%20%28single-precision%29))
  (bind _self self)
  (bind _returnvalue (Transformation|GetActorLocation _self))
  (bind _x (Math|Vector|BreakVector _returnvalue))
  (bind _inrange (CallFunction|CheckinRange (Transformation|GetActorLocation self) (Transformation|GetActorLocation (Game|GetPlayerCharacter 0)) 1.2e+03))
  (if _inrange
    (bind _updatedcurrent (CallFunction|ChangeFlipbook (Variables|Default|GetActiveFlipbook) "Attack"))
    (Variables|Default|SetActiveFlipbook _updatedcurrent)
    (if (< (- (.X (Math|Vector|BreakVector (Transformation|GetActorLocation (Game|GetPlayerCharacter 0)))) (.X (Math|Vector|BreakVector (Transformation|GetActorLocation self)))) 0.0)
      (Variables|Default|SetDirection -1.0)
      (if (>= (- _x (.X (Math|Vector|BreakVector (Variables|Default|GetLeftPoint)))) 1e+02)
        (CallFunction|Move :!label _label))
      (else
        (Variables|Default|SetDirection 1.0)
        (if (>= (- (.X (Math|Vector|BreakVector (Variables|Default|GetRightPoint))) _x) -1e+02)
          (goto _label))))
    (else
      (bind _updatedcurrent_2 (CallFunction|ChangeFlipbook (Variables|Default|GetActiveFlipbook) "Walk"))
      (Variables|Default|SetActiveFlipbook _updatedcurrent_2)
      (CallFunction|Move))))

(event EventBeginPlay)

(fn ConstructionScript
  (bind _pointa (Variables|Default|GetPointA))
  (bind _pointb (Variables|Default|GetPointB))
  (bind _returnvalue (Transformation|GetActorLocation _pointa))
  (bind _returnvalue_2 (Transformation|GetActorLocation _pointb))
  (Math|Float|CompareFloat (.X (Math|Vector|BreakVector _returnvalue)) (.X (Math|Vector|BreakVector _returnvalue_2))
    (:>
      (Variables|Default|SetRightPoint _returnvalue)
      (Variables|Default|SetLeftPoint _returnvalue_2))
    (:<
      (Variables|Default|SetRightPoint _returnvalue_2)
      (Variables|Default|SetLeftPoint _returnvalue)))
  (switch Utilities|FlowControl|Switch|SwitchonEnemyTypeEnum (Variables|Default|GetEnemyType)
    (:NewEnumerator0
      (Variables|Default|SetWalkFlipbook "/Game/Sprites/Characters/BlacksmithWalk.BlacksmithWalk")
      (Variables|Default|SetIdleFlipbook "/Game/Sprites/Characters/BlacksmithIdle.BlacksmithIdle")
      (Variables|Default|SetAttackFlipbook "/Game/Sprites/Characters/PlaceHolders/AttackPlaceHolder.AttackPlaceHolder")
      (Sprite|SetFlipbook (Variables|Default|GetSprite) (Variables|Default|GetWalkFlipbook)))))

(fn SwitchDirection
  (if (== (Variables|Default|GetDirection) 1.0)
    (Variables|Default|SetDirection -1.0)
    (else
      (Variables|Default|SetDirection 1.0))))

(fn CheckinRange
  (params (Position%20A :type Vector) (Position%20B :type Vector) (Distance :type Float%20%28single-precision%29))
  (bind (_x _y _z) (Math|Vector|BreakVector Position%20A))
  (bind (_x_2 _y_2 _z_2) (Math|Vector|BreakVector Position%20B))
  (return (<= (Math|Float|Sqrt (+ (Math|Float|Square (- _x _x_2)) (Math|Float|Square (- _z _z_2)))) Distance)))

(fn ChangeFlipbook
  (params (Current :type Name :default "None") (New :type Name :default "None"))
  (if (Utilities|Name|Equal(Name) Current New)
    (return New)
    (else
      (switch name New
        (:Walk
          (LocalVariables|SetNewFlipbook (Variables|Default|GetWalkFlipbook)))
        (:Idle
          (LocalVariables|SetNewFlipbook (Variables|Default|GetIdleFlipbook)))
        (:attack
          (LocalVariables|SetNewFlipbook (Variables|Default|GetAttackFlipbook))))
      (Sprite|SetFlipbook (Variables|Default|GetSprite) (LocalVariables|GetNewFlipbook)))))

(fn Move
  (if (== (Variables|Default|GetDirection) 1.0)
    (Transformation|SetActorRelativeRotation "0, 0, 0")
    (else
      (Transformation|SetActorRelativeRotation "0,180.000000, 0")))
  (Pawn|Input|AddMovementInput "1.000000, 0, 0" (Variables|Default|GetDirection)))